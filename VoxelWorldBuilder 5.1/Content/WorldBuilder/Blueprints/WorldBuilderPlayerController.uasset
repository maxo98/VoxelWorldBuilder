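; Player controller for a world-building mode that places, selects and deletes cubes and drives the CameraController pawn's orbit, pitch and zoom.
; In placement mode, a preview actor follows a cursor or camera-forward trace, snapped to a grid that the mouse wheel scales with the cube.
; Clicking spawns cubes if placement is valid.
; Outside placement, clicks toggle selection flags in the CubesList map, which Delete uses to destroy selected cubes.
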(event EventTick
  (params (DeltaSeconds :type Float%20%28single-precision%29))
  (if (Variables|Default|GetPlacementModeEnabled)
    (CallFunction|UpdatePlacement)))

(event EventBeginPlay
  (bind _ascamera_controller (Utilities|Casting|CastToCameraController (Pawn|GetControlledPawn)))
  (Variables|Default|SetPlayerCharacter _ascamera_controller)
  (Variables|Default|SetCurrentGridSize (Variables|Default|GetDefaultGridSize))
  (Variables|Default|SetPlacementModeEnabled true)
  (CallFunction|SetPlacementModeEnabled))

(event Input|ActionEvents|InputActionEnableBuild
  (params (Key :type Key%20Structure :default "None"))
  ;[1 1 1] Inputs
  (:Pressed
    (Variables|Default|SetPlacementModeEnabled (not (Variables|Default|GetPlacementModeEnabled)))
    (CallFunction|SetPlacementModeEnabled)))

(event Input|ActionEvents|InputActionMouseLeftClick
  (params (Key :type Key%20Structure :default "None"))
  ;[1 1 1] Inputs
  (:Pressed
    (if (Variables|Default|GetPlacementModeEnabled)
      (CallFunction|SpawnCube)
      (elif (Variables|Default|GetHasMouseControl)
        (CallFunction|OnMouseClick)))))

(event Input|ActionEvents|InputActionCameraMouseControl
  (params (Key :type Key%20Structure :default "None"))
  ;[1 1 1] Inputs
  (:Pressed
    (Variables|Default|SetHasCameraMouseControl true)
    (bind _output_get (Variables|Default|SetHasMouseControl false))
    (Variables|Default|SetbShowMouseCursor _output_get)
    (Variables|Default|SetPlacementModeEnabled false)
    (CallFunction|SetPlacementModeEnabled))
  (:Released
    (Variables|Default|SetHasCameraMouseControl false)
    (bind _output_get_2 (Variables|Default|SetHasMouseControl true))
    (Variables|Default|SetbShowMouseCursor _output_get_2)
    (Variables|Default|SetPlacementModeEnabled true)
    (CallFunction|SetPlacementModeEnabled)))

(event Input|ActionEvents|InputActionDeleteSelection
  (params (Key :type Key%20Structure :default "None"))
  ;[1 1 1] Inputs
  (:Pressed
    (bind _keys (Utilities|Map|Keys (Variables|Default|GetCubesList)))
    (for _array_element _keys
      (if (and (.Value (Utilities|Map|Find (Variables|Default|GetCubesList) _array_element)) (.ReturnValue (Utilities|Map|Find (Variables|Default|GetCubesList) _array_element)))
        (Utilities|Map|Remove (Variables|Default|GetCubesList) _array_element)
        (Actor|DestroyActor (Components|GetOwner _array_element))))))

(event Input|ActionEvents|InputActionToggleMouseControl
  (params (Key :type Key%20Structure :default "None"))
  ;[1 1 1] Inputs
  (:Pressed
    (if (Variables|Default|GetHasMouseControl)
      (bind _output_get (Variables|Default|SetHasMouseControl false))
      (Variables|Default|SetbShowMouseCursor _output_get)
      (else
        (bind _output_get_2 (Variables|Default|SetHasMouseControl true))
        (Variables|Default|SetbShowMouseCursor _output_get_2)))))

(event Input|AxisEvents|InputAxisMouseX
  (params (AxisValue :type Float%20%28single-precision%29))
  ;[1 1 1] Inputs
  (if (and (Variables|Default|GetHasCameraMouseControl) (not (Variables|Default|GetHasMouseControl)))
    (Default|CameraOrbit (Variables|Default|GetPlayerCharacter) AxisValue)))

(event Input|AxisEvents|InputAxisMouseY
  (params (AxisValue :type Float%20%28single-precision%29))
  ;[1 1 1] Inputs
  (if (and (Variables|Default|GetHasCameraMouseControl) (not (Variables|Default|GetHasMouseControl)))
    (Default|PitchCamera (Variables|Default|GetPlayerCharacter) AxisValue)))

(event Input|AxisEvents|InputAxisMouseWheel
  (params (AxisValue :type Float%20%28single-precision%29))
  ;[1 1 1] Inputs
  (if (Variables|Default|GetPlacementModeEnabled)
    (CallFunction|ChangeCubeandGridSize AxisValue)
    (else
      (Default|ChangeCameraDistance (Variables|Default|GetPlayerCharacter) AxisValue))))

(fn ConstructionScript)

(fn SetPlacementModeEnabled
  (if (Variables|Default|GetPlacementModeEnabled)
    (bind _returnvalue (Game|SpawnActorfromClass (Variables|Default|GetPlaceableActorType) (Math|Transform|MakeTransform "0, 0,-1000.000000") "AlwaysSpawn" 0 0))
    (bind _output_get (Variables|Default|SetPlaceableActor _returnvalue))
    (Utilities|IsValid (Actor|GetComponentbyClass _output_get "/Game/WorldBuilder/Objects/Component/ClickableComponent.ClickableComponent_C")
      (:Is%20Valid
        (Default|InPlacementMode (Actor|GetComponentbyClass _output_get "/Game/WorldBuilder/Objects/Component/ClickableComponent.ClickableComponent_C")))
      (:Is%20Not%20Valid
        _))
    (AddComponent|AddPlaceableComponent (Variables|Default|GetPlaceableActor))
    (else
      (Utilities|IsValid (Variables|Default|GetPlaceableActor)
        (:Is%20Valid
          (Actor|DestroyActor (Variables|Default|GetPlaceableActor)))))))

(fn UpdatePlacement
  (bind (_worldlocation _worlddirection) (Game|Player|ConvertMouseLocationToWorldSpace))
  (bind _playercharacter (Variables|Default|GetPlayerCharacter))
  (bind _camera (Variables|/Game/WorldBuilder/Blueprints/CameraController.CameraController_C|GetCamera _playercharacter))
  (bind _returnvalue (Transformation|GetWorldLocation _camera))
  (if (not (Variables|Default|GetHasMouseControl))
    (bind _outhit (Collision|LineTraceByChannel _returnvalue (+ _returnvalue (* (Math|Vector|GetForwardVector _camera) 1e+05)) "TraceTypeQuery3" false (Utilities|Array|MakeArray _playercharacter) "None"))
    (if (.bblockinghit _outhit)
      (Transformation|SetActorLocation (Variables|Default|GetPlaceableActor) (Class|KismetMathLibrary|VectorSnappedtoGrid (.location _outhit) (Variables|Default|GetCurrentGridSize)) false false))
    (else
      (bind _outhit_2 (Collision|LineTraceByChannel _worldlocation (+ _worldlocation (* _worlddirection 1e+05)) "TraceTypeQuery3" false 0 "None"))
      (if (.bblockinghit _outhit_2)
        (Transformation|SetActorLocation (Variables|Default|GetPlaceableActor) (Class|KismetMathLibrary|VectorSnappedtoGrid (.location _outhit_2) (Variables|Default|GetCurrentGridSize)) false false)))))

(fn SpawnCube
  (bind _placeableactor (Variables|Default|GetPlaceableActor))
  (bind _returnvalue (Actor|GetComponentbyClass _placeableactor "/Game/WorldBuilder/Objects/Component/PlaceableComponent.PlaceableComponent_C"))
  (Utilities|IsValid _returnvalue
    (:Is%20Valid
      (if (Variables|/Game/WorldBuilder/Objects/Component/PlaceableComponent.PlaceableComponent_C|GetIsPlacementValid _returnvalue)
        (bind _returnvalue_2 (Game|SpawnActorfromClass (Variables|Default|GetPlaceableActorType) (Transformation|GetActorTransform (Variables|Default|GetPlaceableActor)) "Undefined" 0 0))
        (bind _asplaceable_cube_bp (Utilities|Casting|CastToPlaceableCubeBP _returnvalue_2))
        (bind _clickablecomponent (Default|Placed _asplaceable_cube_bp))
        (Utilities|Map|Add (Variables|Default|GetCubesList) _clickablecomponent false)))))

(fn OnMouseClick
  (bind (_worldlocation _worlddirection) (Game|Player|ConvertMouseLocationToWorldSpace))
  (bind _cubeslist (Variables|Default|GetCubesList))
  (bind _outhit (Collision|LineTraceByChannel _worldlocation (+ _worldlocation (* _worlddirection 1e+05)) "TraceTypeQuery3" false 0 "None"))
  (Utilities|IsValid (Actor|GetComponentbyClass (.hitactor _outhit) "/Game/WorldBuilder/Objects/Component/ClickableComponent.ClickableComponent_C")
    (:Is%20Valid
      (Default|OnMouseClicked (Actor|GetComponentbyClass (.hitactor _outhit) "/Game/WorldBuilder/Objects/Component/ClickableComponent.ClickableComponent_C"))
      (if (.ReturnValue (Utilities|Map|Find _cubeslist (Actor|GetComponentbyClass (.hitactor _outhit) "/Game/WorldBuilder/Objects/Component/ClickableComponent.ClickableComponent_C")))
        (Utilities|Map|Add _cubeslist (Actor|GetComponentbyClass (.hitactor _outhit) "/Game/WorldBuilder/Objects/Component/ClickableComponent.ClickableComponent_C") (not (.Value (Utilities|Map|Find _cubeslist (Actor|GetComponentbyClass (.hitactor _outhit) "/Game/WorldBuilder/Objects/Component/ClickableComponent.ClickableComponent_C")))))))))

(fn ChangeCubeandGridSize
  (params (NewSize :type Float%20%28double-precision%29))
  (if (!= NewSize 0.0)
    (bind _output_get (Variables|Default|SetCubeSize (Math|Float|Clamp(Float) (+ (Variables|Default|GetCubeSize) (* (Variables|Default|GetCubeResizeSpeed) NewSize)) 0.25 2.0)))
    (Variables|Default|SetCurrentGridSize (* (Variables|Default|GetDefaultGridSize) _output_get))
    (Transformation|SetActorScale3D (Variables|Default|GetPlaceableActor) (Math|Vector|MakeVector (Variables|Default|GetCubeSize) (Variables|Default|GetCubeSize) (Variables|Default|GetCubeSize)))))