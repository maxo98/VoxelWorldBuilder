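; Player character for the World Builder, with camera-relative movement and an orbit, pitch and zoom camera on a spring arm.
; Orbit input yaws the arm, pitch input is clamped between angle limits, and zoom input sets a clamped target length.
; Tick eases the arm toward that length and scales max walk speed by its ratio to the minimum distance, so movement is faster when zoomed out.
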(event Custom|CameraOrbit
  (params (Magnitude :type Float%20%28double-precision%29))
  ;[1 1 1] Controls
  (Transformation|AddWorldRotation (Variables|Default|GetSpringArm) (Math|Rotator|MakeRotator 0.0 0.0 (* Magnitude (Variables|CameraMovements|GetOrbitSpeed))) false false))

(event Custom|ChangeCameraDistance
  (params (Magnitude :type Float%20%28double-precision%29))
  ;[1 1 1] Controls
  (if (!= Magnitude 0.0)
    (Variables|CameraMovements|SetTargetSpringLength (Math|Float|Clamp(Float) (+ (* Magnitude (Variables|CameraMovements|GetCamDistanceSpeed)) (Variables|/Script/Engine.SpringArmComponent|GetTargetArmLength (Variables|Default|GetSpringArm))) (Variables|CameraMovements|GetCamDistanceMin) (Variables|CameraMovements|GetCamDistanceMax)))))

(event Custom|MoveForward
  (params (Magnitude :type Float%20%28double-precision%29))
  ;[1 1 1] Controls
  (Pawn|Input|AddMovementInput (Math|Vector|GetForwardVector (Variables|Default|GetCamera)) Magnitude false))

(event Custom|PitchCamera
  (params (Magnitude :type Float%20%28double-precision%29))
  (bind _springarm (Variables|Default|GetSpringArm))
  (bind _returnvalue (Transformation|GetWorldRotation _springarm))
  ;[1 1 1] Controls
  (Transformation|SetWorldRotation (Variables|Default|GetSpringArm) (Math|Rotator|MakeRotator (.roll _returnvalue) (Math|Float|ClampAngle (+ (* Magnitude (Variables|CameraMovements|GetOrbitSpeed)) (.pitch _returnvalue)) (Variables|CameraMovements|GetMinPitch%20Angle%20Degrees) (Variables|CameraMovements|GetMax%20Pitch%20Angle%20Degrees)) (.yaw _returnvalue)) false false))

(event Custom|MoveRight
  (params (Magnitude :type Float%20%28double-precision%29))
  ;[1 1 1] Controls
  (Pawn|Input|AddMovementInput (Math|Vector|GetRightVector (Variables|Default|GetCamera)) Magnitude false))

(event EventBeginPlay
  (Variables|CameraMovements|SetInitialMovementSpeed (Variables|/Script/Engine.CharacterMovementComponent|GetMaxWalkSpeed (Variables|Character|GetCharacterMovement)))
  (Variables|CameraMovements|SetTargetSpringLength (Variables|/Script/Engine.SpringArmComponent|GetTargetArmLength (Variables|Default|GetSpringArm)))
  (CallFunction|UpdateMovementSpeedfromCameraDistance))

(event EventTick
  (params (DeltaSeconds :type Float%20%28single-precision%29))
  (CallFunction|UpdateCameraDistanceonTick DeltaSeconds)
  (CallFunction|UpdateMovementSpeedfromCameraDistance))

(fn ConstructionScript)

(fn UpdateMovementSpeedfromCameraDistance
  (Variables|/Script/Engine.CharacterMovementComponent|SetMaxWalkSpeed (Variables|Character|GetCharacterMovement) (* (/ (Variables|/Script/Engine.SpringArmComponent|GetTargetArmLength (Variables|Default|GetSpringArm)) (Variables|CameraMovements|GetCamDistanceMin)) (Variables|CameraMovements|GetInitialMovementSpeed))))

(fn UpdateCameraDistanceonTick
  (params (DeltaTime :type Float%20%28double-precision%29))
  (Variables|/Script/Engine.SpringArmComponent|SetTargetArmLength (Variables|Default|GetSpringArm) (Math|Interpolation|FInterpTo (Variables|/Script/Engine.SpringArmComponent|GetTargetArmLength (Variables|Default|GetSpringArm)) (Variables|CameraMovements|GetTargetSpringLength) DeltaTime 5.0)))