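; Game mode for a voxel world builder that saves and loads cube scenes as files in the project's Saves folder.
; SaveGame serializes each cube in the player controller's CubesList as scaled-down position, material color and scale into one string, using a date-and-hour autosave name when none is given.
; LoadGame clears the scene, parses each line, maps scale indices through SetScale and respawns cubes via the controller's CreateCube.
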(event EventBeginPlay
  (Variables|Default|SetFilePath (Utilities|String|Append (Class|KismetSystemLibrary|GetProjectDirectory) "Saves/")))

(fn ConstructionScript)

(fn SaveGame
  (params (FileName :type String))
  (bind _returnvalue (Math|DateTime|Now))
  (bind _divider (Variables|Default|Getdivider))
  (if (Utilities|Array|IsEmpty FileName)
    (bind _output_get (Variables|Default|SetFilePath (Utilities|String|Append (Variables|Default|GetFilePath) "auto_savefile_" (Utilities|String|ToString(Integer) (.year _returnvalue)) "_" (Utilities|String|ToString(Integer) (.month _returnvalue)) "_" (Utilities|String|ToString(Integer) (.day _returnvalue)) "_" (Utilities|String|ToString(Integer) (.hour _returnvalue)) ".txt")))
    (else
      (Variables|Default|SetFilePath (Utilities|String|Append (Variables|Default|GetFilePath) FileName ".txt"))))
  (Variables|Default|SetVoxelString "")
  (Class|ReadWritePluginBPLibrary|DeleteFile _output_get)
  (bind _asworld_builder_player_controller (Utilities|Casting|CastToWorldBuilderPlayerController (Game|GetPlayerController 0)))
  (bind _keys (Utilities|Map|Keys (Variables|/Game/WorldBuilder/Blueprints/WorldBuilderPlayerController.WorldBuilderPlayerController_C|GetCubesList _asworld_builder_player_controller)))
  (for _array_element _keys
    (bind _asplaceable_cube_bp (Utilities|Casting|CastToPlaceableCubeBP (Components|GetOwner _array_element)))
    (bind _asmaterial_instance_dynamic (Utilities|Casting|CastToMaterialInstanceDynamic (Rendering|Material|GetMaterial (Variables|/Game/WorldBuilder/Objects/PlaceableCubeBP.PlaceableCubeBP_C|GetCube _asplaceable_cube_bp) 0)))
    (bind _returnvalue_2 (Rendering|Material|GetVectorParameterValue _asmaterial_instance_dynamic "Color" :!class /Script/Engine.MaterialInstanceDynamic))
    (bind _scalevalue (Default|GetVoxelScale _asplaceable_cube_bp))
    (Variables|Default|SetVoxelString (Utilities|String|Append (Variables|Default|GetVoxelString) (Class|VictoryBPFunctionLibrary|StringCombineStringsMulti (Utilities|String|ToString(Float) (/ (.x (Transformation|GetActorLocation _asplaceable_cube_bp)) _divider)) (Utilities|String|ToString(Float) (/ (.y (Transformation|GetActorLocation _asplaceable_cube_bp)) _divider)) (Utilities|String|ToString(Float) (/ (.z (Transformation|GetActorLocation _asplaceable_cube_bp)) _divider)) (Utilities|String|ToString(Float) (.r _returnvalue_2)) (Utilities|String|ToString(Float) (.g _returnvalue_2)) (Utilities|String|ToString(Float) (.b _returnvalue_2)) (Utilities|String|ToString(Integer) _scalevalue) " 
"))))
  (Class|ReadWritePluginBPLibrary|SaveStringtoFile (Variables|Default|GetFilePath) (Variables|Default|GetVoxelString))
  (Variables|Default|SetFilePath (Utilities|String|Append (Class|KismetSystemLibrary|GetProjectDirectory) "Saves/")))

(fn LoadGame
  (params (FilePath :type String))
  (bind _asworld_builder_player_controller (Utilities|Casting|CastToWorldBuilderPlayerController (Game|GetPlayerController 0)))
  (Default|CleanScene _asworld_builder_player_controller)
  (bind _returnvalue (Class|ReadWritePluginBPLibrary|ReadStringfromFile FilePath))
  (bind _output_get (LocalVariables|SetLines (Utilities|String|ParseIntoArray _returnvalue " 
")))
  (for _array_element _output_get
    (bind _output_get_2 (LocalVariables|SetVoxelLine (Utilities|String|ParseIntoArray _array_element " ")))
    (LocalVariables|SetVoxelLocation (Math|Vector|MakeVector (* (Math|Conversions|ToFloat(Integer) (Utilities|Array|Get(acopy) _output_get_2)) 1e+02) (* (Math|Conversions|ToFloat(Integer) (Utilities|Array|Get(acopy) _output_get_2 1)) 1e+02) (* (Math|Conversions|ToFloat(Integer) (Utilities|Array|Get(acopy) _output_get_2 2)) 1e+02)))
    (LocalVariables|SetVoxelColor (Utilities|Struct|MakeLinearColor (Math|Conversions|ToFloat(Integer) (Utilities|Array|Get(acopy) (LocalVariables|GetVoxelLine) 3)) (Math|Conversions|ToFloat(Integer) (Utilities|Array|Get(acopy) (LocalVariables|GetVoxelLine) 4)) (Math|Conversions|ToFloat(Integer) (Utilities|Array|Get(acopy) (LocalVariables|GetVoxelLine) 5)) 1.0))
    (bind _scalevalue (CallFunction|SetScale (Math|Conversions|ToInteger(Byte) (Utilities|Array|Get(acopy) (LocalVariables|GetVoxelLine) 6))))
    (LocalVariables|SetVoxelScale _scalevalue)
    (bind _asworld_builder_player_controller_2 (Utilities|Casting|CastToWorldBuilderPlayerController (Game|GetPlayerController 0)))
    (Default|CreateCube _asworld_builder_player_controller_2 (LocalVariables|GetVoxelLocation) (LocalVariables|GetVoxelColor) (LocalVariables|GetVoxelScale))))

(fn SetScale
  (params (newScale :type Integer))
  (switch int newScale
    (:Default
      _)
    (:0
      _)
    (:1
      (return 4.0))
    (:2
      (return 2.0))
    (:3
      _)
    (:4
      (return 0.5))
    (:5
      (return 0.25))
    (:6
      (return 0.125)))
  (return 1.0))