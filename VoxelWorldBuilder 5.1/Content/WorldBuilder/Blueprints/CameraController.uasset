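; Camera pawn for the world builder that moves, orbits, pitches and zooms the view around a spring arm.
; Input events drive camera-relative movement, clamped height changes with a reset to starting height, and clamped pitch.
; Zoom sets a clamped target arm length that Tick smoothly interpolates toward.
; On BeginPlay it also opens the main menu widget, passing the player controller to the voxel world builder interface.
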(event Custom|CameraOrbit
  (params (Magnitude :type Float%20%28double-precision%29))
  ;[1 1 1] Controls
  (Transformation|AddWorldRotation (Variables|Default|GetSpringArm) (Math|Rotator|MakeRotator 0.0 0.0 (* Magnitude (Variables|Default|GetOrbitSpeed))) false false))

(event Custom|ChangeCameraDistance
  (params (Magnitude :type Float%20%28double-precision%29))
  ;[1 1 1] Controls
  (if (!= Magnitude 0.0)
    (Variables|Default|SetTargetSpringLength (Math|Float|Clamp(Float) (+ (* Magnitude (Variables|Default|GetCamDistanceSpeed)) (Variables|/Script/Engine.SpringArmComponent|GetTargetArmLength (Variables|Default|GetSpringArm))) (Variables|Default|GetCamDistanceMin) (Variables|Default|GetCamDistanceMax)))))

(event Custom|MoveForward
  (params (Magnitude :type Float%20%28double-precision%29))
  ;[1 1 1] Controls
  (Pawn|Input|AddMovementInput (Math|Vector|GetForwardVector (Variables|Default|GetCamera)) Magnitude false))

(event Custom|PitchCamera
  (params (Magnitude :type Float%20%28double-precision%29))
  (bind _springarm (Variables|Default|GetSpringArm))
  (bind _returnvalue (Transformation|GetWorldRotation _springarm))
  ;[1 1 1] Controls
  (Transformation|SetWorldRotation (Variables|Default|GetSpringArm) (Math|Rotator|MakeRotator (.roll _returnvalue) (Math|Float|ClampAngle (+ (* Magnitude (Variables|Default|GetOrbitSpeed)) (.pitch _returnvalue)) (Variables|Default|GetMinPitch%20Angle%20Degrees) (Variables|Default|GetMax%20Pitch%20Angle%20Degrees)) (.yaw _returnvalue)) false false))

(event Custom|MoveRight
  (params (Magnitude :type Float%20%28double-precision%29))
  ;[1 1 1] Controls
  (Pawn|Input|AddMovementInput (Math|Vector|GetRightVector (Variables|Default|GetCamera)) Magnitude false))

(event Custom|Move%20Up%20/down
  (params (Magnitude :type Float%20%28double-precision%29))
  (bind _returnvalue (Transformation|GetActorLocation))
  ;[1 1 1] Controls
  (Transformation|SetActorLocation (Math|Vector|MakeVector (.x _returnvalue) (.y _returnvalue) (Math|Float|Clamp(Float) (+ (* Magnitude (Variables|Default|GetMovementSpeed)) (.z _returnvalue)) 2e+02 1e+03)) false false))

(event Custom|ResetPosition
  (bind _returnvalue (Transformation|GetActorLocation))
  ;[1 1 1] Controls
  (Transformation|SetActorLocation (Math|Vector|MakeVector (.x _returnvalue) (.y _returnvalue) (Variables|Default|GetInitialHeight)) false false))

(event EventBeginPlay
  (Variables|Default|SetTargetSpringLength (Variables|/Script/Engine.SpringArmComponent|GetTargetArmLength (Variables|Default|GetSpringArm)))
  (CallFunction|ShowUI "/Game/WorldBuilder/UI/MainMenuUI.MainMenuUI_C")
  (Variables|Default|SetInitialHeight (.z (Transformation|GetActorLocation))))

(event EventTick
  (params (DeltaSeconds :type Float%20%28single-precision%29))
  (CallFunction|UpdateCameraDistanceonTick DeltaSeconds))

(fn ConstructionScript)

(fn UpdateCameraDistanceonTick
  (params (DeltaTime :type Float%20%28double-precision%29))
  (Variables|/Script/Engine.SpringArmComponent|SetTargetArmLength (Variables|Default|GetSpringArm) (Math|Interpolation|FInterpTo (Variables|/Script/Engine.SpringArmComponent|GetTargetArmLength (Variables|Default|GetSpringArm)) (Variables|Default|GetTargetSpringLength) DeltaTime 5.0)))

(fn ShowUI
  (params (WidgetToLoad :type Voxel%20World%20Builder%20Interface%20Class%20Reference))
  (bind _returnvalue (UserInterface|CreateWidget WidgetToLoad (Game|GetPlayerController 0)))
  (bind _output_get (Variables|Default|SetCurrentInterfaceDisplayed _returnvalue))
  (bind _asvoxel_world_builder_interface (Utilities|Casting|CastToVoxelWorldBuilderInterface _output_get))
  (bind _asworld_builder_player_controller (Utilities|Casting|CastToWorldBuilderPlayerController (Game|GetPlayerController 0)))
  (Variables|/Game/WorldBuilder/UI/VoxelWorldBuilderInterface.VoxelWorldBuilderInterface_C|SetPlayerController _asvoxel_world_builder_interface _asworld_builder_player_controller)
  (UserInterface|Viewport|AddtoViewport _returnvalue 0))

(fn RemoveUI
  (Viewport|RemoveAllWidgets))