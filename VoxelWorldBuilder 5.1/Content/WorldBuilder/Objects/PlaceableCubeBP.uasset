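; PlaceableCubeBP is a world-builder cube object that takes a color and becomes clickable once placed.
; Placed applies a colored dynamic instance of the material cached at BeginPlay, enables query-only collision blocking GameTraceChannel1, then adds and returns a clickable component.
; Two helpers convert between actor scale and discrete voxel size levels, with higher levels meaning smaller cubes.
; SetVoxelScale only returns the scale value and does not resize the actor.
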(event EventBeginPlay
  (Variables|Default|SetDefaultMaterial "/Game/WorldBuilder/Materials/PlacedCubeMaterial.PlacedCubeMaterial"))

(fn ConstructionScript)

(fn Placed
  (params (NewColor :type Color%20Structure))
  (bind _cube (Variables|Default|GetCube))
  (bind _returnvalue (Rendering|Material|CreateDynamicMaterialInstance _cube 0 (Variables|Default|GetDefaultMaterial) "None" :!class /Script/Engine.PrimitiveComponent))
  (Rendering|Material|SetVectorParameterValue _returnvalue "Color" (Math|Conversions|ToLinearColor(Color) NewColor) :!class /Script/Engine.MaterialInstanceDynamic)
  (Collision|SetCollisionResponsetoChannel _cube "ECC_GameTraceChannel1" "ECR_Block")
  (Collision|SetCollisionEnabled _cube "QueryOnly")
  (bind _returnvalue_2 (AddComponent|AddClickableComponent))
  (bind _output_get (Variables|Default|SetClickableComponent _returnvalue_2))
  (return _output_get))

(fn GetVoxelScale
  (bind _output_get (LocalVariables|SetCurrentScale (.x (Transformation|GetActorScale3D))))
  (if (< _output_get 0.5)
    (return 5)
    (elif (< (LocalVariables|GetCurrentScale) 1.0)
      (return 4)
      (elif (< (LocalVariables|GetCurrentScale) 2.0)
        (return 3)
        (elif (< (LocalVariables|GetCurrentScale) 4.0)
          (return 2)
          (else
            (return 1)))))))

(fn SetVoxelScale
  (params (Scale :type Integer))
  (switch int Scale
    (:Default
      _)
    (:0
      _)
    (:1
      (return 4.0))
    (:2
      (return 2.0))
    (:3
      _)
    (:4
      (return 0.5))
    (:5
      (return 0.25)))
  (return 1.0))