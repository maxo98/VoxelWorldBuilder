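; Player controller for the WorldBuilder game that turns input into movement and camera control on the possessed WorldBuilderPlayerBP pawn.
; It caches the pawn on BeginPlay and forwards move, orbit, pitch and camera distance axes to it.
; Mouse movement orbits and pitches the camera only while the camera mouse control action is held and cursor mode is off.
; A toggle action switches cursor mode, enabling the visible cursor, click and mouse-over events.
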(event EventBeginPlay
  (bind _asworld_builder_player_bp (Utilities|Casting|CastToWorldBuilderPlayerBP (Pawn|GetControlledPawn)))
  (Variables|Default|SetPlayerCharacter _asworld_builder_player_bp))

(event Input|ActionEvents|InputActionCameraMouseControl
  (params (Key :type Key%20Structure :default "None"))
  (:Pressed
    (Variables|Default|SetHasCameraMouseControl true))
  (:Released
    (Variables|Default|SetHasCameraMouseControl false)))

(event Input|ActionEvents|InputActionToggleMouseControl
  (params (Key :type Key%20Structure :default "None"))
  (:Pressed
    (if (Variables|Default|GetHasMouseControl)
      (Variables|Default|SetHasMouseControl false)
      (Variables|Default|SetbShowMouseCursor false)
      (Variables|Default|SetbEnableClickEvents false)
      (Variables|Default|SetbEnableMouseOverEvents false)
      (else
        (Variables|Default|SetHasMouseControl true)
        (Variables|Default|SetbShowMouseCursor true)
        (Variables|Default|SetbEnableClickEvents true)
        (Variables|Default|SetbEnableMouseOverEvents true)))))

(event Input|AxisEvents|InputAxisOrbitRight/Left
  (params (AxisValue :type Float%20%28single-precision%29))
  (Default|CameraOrbit (Variables|Default|GetPlayerCharacter) AxisValue))

(event Input|AxisEvents|InputAxisMoveForward/Backward
  (params (AxisValue :type Float%20%28single-precision%29))
  (Default|MoveForward (Variables|Default|GetPlayerCharacter) AxisValue))

(event Input|AxisEvents|InputAxisMoveRight/Left
  (params (AxisValue :type Float%20%28single-precision%29))
  (Default|MoveRight (Variables|Default|GetPlayerCharacter) AxisValue))

(event Input|AxisEvents|InputAxisCameraPitch
  (params (AxisValue :type Float%20%28single-precision%29))
  (Default|PitchCamera (Variables|Default|GetPlayerCharacter) AxisValue))

(event Input|AxisEvents|InputAxisCameraDistance
  (params (AxisValue :type Float%20%28single-precision%29))
  (Default|ChangeCameraDistance (Variables|Default|GetPlayerCharacter) AxisValue))

(event Input|AxisEvents|InputAxisMouseX
  (params (AxisValue :type Float%20%28single-precision%29))
  (if (and (Variables|Default|GetHasCameraMouseControl) (not (Variables|Default|GetHasMouseControl)))
    (Default|CameraOrbit (Variables|Default|GetPlayerCharacter) AxisValue)))

(event Input|AxisEvents|InputAxisMouseY
  (params (AxisValue :type Float%20%28single-precision%29))
  (if (and (Variables|Default|GetHasCameraMouseControl) (not (Variables|Default|GetHasMouseControl)))
    (Default|PitchCamera (Variables|Default|GetPlayerCharacter) AxisValue)))

(fn ConstructionScript)